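; BP_LeftDoor is a left door actor that switches between open and closed whenever something begins overlapping its Box trigger.
; The overlap calls an open/close event that checks IsDoorOpen, instantly moves SMLeftDoor on X, then flips the flag.
; Both branches subtract CloseByAmount or OpenByAmount from the mesh's world X and apply the result as relative location.
; Print strings trace each branch for debugging.
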(event OnComponentBeginOverlap(Box)
  (params (OverlappedComponent :type Primitive%20Component%20Object%20Reference) (OtherActor :type Actor%20Object%20Reference) (OtherComp :type Primitive%20Component%20Object%20Reference) (OtherBodyIndex :type Integer) (bFromSweep :type Boolean) (SweepResult :type Hit%20Result%20Structure%20%28by%20ref%29))
  (CallFunction|Open/CloseDoor))

(event Custom|Open/CloseDoor
  (Development|PrintString "Ok will do")
  (if (Variables|Default|GetIsDoorOpen)
    (Development|PrintString "opening")
    (Transformation|SetRelativeLocation (Variables|Default|GetSM_LeftDoor) (Math|Vector|MakeVector (- (.x (Transformation|GetWorldLocation (Variables|Default|GetSM_LeftDoor))) (Variables|Default|GetCloseByAmount)) 0.0 0.0) false false)
    (Variables|Default|SetIsDoorOpen false)
    (Development|PrintString "No")
    (else
      (Development|PrintString "closing")
      (Transformation|SetRelativeLocation (Variables|Default|GetSM_LeftDoor) (Math|Vector|MakeVector (- (.x (Transformation|GetWorldLocation (Variables|Default|GetSM_LeftDoor))) (Variables|Default|GetOpenByAmount)) 0.0 0.0) false false)
      (Variables|Default|SetIsDoorOpen true)
      (Development|PrintString "Hello"))))

(fn ConstructionScript)