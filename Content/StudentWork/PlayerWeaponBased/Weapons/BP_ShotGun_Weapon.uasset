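; Shotgun weapon Blueprint for a tank that fires a three-projectile spread when triggered.
; Triggered spawns a BP_ShotGun_Projectile at the location and rotation of each of the tank's three direction arrow components, so those arrows define the spread.
; A Cooldown flag blocks further shots until a one-shot timer fires EndCooldown to clear it.
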(event Custom|End%20Cooldown
  (Variables|Default|SetCooldown false))

(event EventTriggered
  (bind _mytank (Variables|Default|GetMyTank))
  (bind _mytank_2 (Variables|Default|GetMyTank))
  (bind _mytank_3 (Variables|Default|GetMyTank))
  (bind _directionarrow (Variables|/Game/Blueprints/BP_PlayerCharacter.BP_PlayerCharacter_C|GetDirectionArrow _mytank))
  (bind _directionarrow1 (Variables|/Game/Blueprints/BP_PlayerCharacter.BP_PlayerCharacter_C|GetDirectionArrow1 _mytank_2))
  (bind _directionarrow2 (Variables|/Game/Blueprints/BP_PlayerCharacter.BP_PlayerCharacter_C|GetDirectionArrow2 _mytank_3))
  (if (not (Variables|Default|GetCooldown))
    (Game|SpawnActorfromClass "/Game/StudentWork/PlayerWeaponBased/Projectiles/BP_ShotGun_Projectile.BP_ShotGun_Projectile_C" (Math|Transform|MakeTransform (Transformation|GetWorldLocation _directionarrow) (Transformation|GetWorldRotation _directionarrow) "1.000000,1.000000,1.000000") "Undefined" "MultiplyWithRoot" 0 0)
    (Game|SpawnActorfromClass "/Game/StudentWork/PlayerWeaponBased/Projectiles/BP_ShotGun_Projectile.BP_ShotGun_Projectile_C" (Math|Transform|MakeTransform (Transformation|GetWorldLocation _directionarrow1) (Transformation|GetWorldRotation _directionarrow1) "1.000000,1.000000,1.000000") "Undefined" "MultiplyWithRoot" 0 0)
    (Game|SpawnActorfromClass "/Game/StudentWork/PlayerWeaponBased/Projectiles/BP_ShotGun_Projectile.BP_ShotGun_Projectile_C" (Math|Transform|MakeTransform (Transformation|GetWorldLocation _directionarrow2) (Transformation|GetWorldRotation _directionarrow2) "1.000000,1.000000,1.000000") "Undefined" "MultiplyWithRoot" 0 0)
    (Variables|Default|SetCooldown true)
    (Utilities|Time|SetTimerbyEvent (delegate Custom|End%20Cooldown) 1.75)))

(fn ConstructionScript
  (|CallParentFunction))